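; Enemy tank character Blueprint that patrols random navigable points around its spawn location and attacks player tanks.
; When aggressive, AI Perception updates trigger aggro, which ends patrolling, changes walk speed and starts a looping timer calling FollowTargetDistance, not defined here.
; PerformAttack faces the target, spawns a projectile, then after a delay fires again or moves back into range, guarded by dead and running-back flags.
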(event OnPerceptionUpdated(AIPerception)
  (params (UpdatedActors :type Array%20of%20Actor%20Object%20References))
  (if (and (not (Variables|Default|GetWasAggroed)) (Variables|Default|GetAgressive))
    (bind _array_element (Utilities|Array|ForEachLoopwithBreak UpdatedActors :!label _label)
      (:LoopBody
        (bind _asbp_char_tank (Utilities|Casting|CastToBp_Char_Tank _array_element))
        (CallFunction|OnAggroPulled _asbp_char_tank)
        (goto _label Break)))))

(event Custom|PerformAttack
  (bind _self self)
  (bind _targetactor (Variables|Default|GetTargetActor))
  (bind _returnvalue (Transformation|GetActorLocation _self))
  (bind _returnvalue_2 (Transformation|GetActorLocation _targetactor))
  (bind _returnvalue_3 (Math|Rotator|FindLookatRotation _returnvalue _returnvalue_2))
  (if (Math|Boolean|ANDBoolean (not (Variables|Default|GetIsDead)) (not (Variables|Default|GetIsRunningBack)) (Variables|Default|GetWasAggroed))
    (Transformation|SetActorRotation _returnvalue_3)
    (Game|SpawnActorfromClass "/Game/BlueSprints/SkillActors/Bp_ActProjectile_Enemy.Bp_ActProjectile_Enemy_C" (Math|Transform|MakeTransform (Transformation|GetWorldLocation (Variables|Default|GetSpawnBullet)) _returnvalue_3 "1,1,1") "Undefined" 0 0)
    (Utilities|FlowControl|Delay 1.5)
    (if (CallFunction|InAttackRange)
      (CallFunction|PerformAttack)
      (else
        (AI|AIMoveTo self "0, 0, 0" (Variables|Default|GetTargetActor) (Variables|Default|GetAtackRange) false
          (:OnSuccess
            _)
          (:OnFail
            _))
        (CallFunction|PerformAttack)))))

(event Custom|Patrol
  (AI|AIMoveTo self (.RandomLocation (Class|NavigationSystemV1|GetRandomPointinNavigableRadius (Variables|Default|GetStartingLocation) (Variables|Default|GetPatrolRadius) 0 0)) 0 5.0 false
    (:OnSuccess
      _)
    (:OnFail
      _))
  (if (Variables|Default|GetIsPatroling)
    (Utilities|FlowControl|Delay (Math|Random|RandomFloatinRange 0.5 2.5))
    (if (Variables|Default|GetIsPatroling)
      (CallFunction|Patrol))))

(event Custom|OnAggroPulled
  (params (Target :type Actor%20Object%20Reference))
  (if (and (not (Variables|Default|GetWasAggroed)) (not (Variables|Default|GetIsRunningBack)))
    (Variables|Default|SetIsPatroling false)
    (Variables|Default|SetWasAggroed true)
    (Variables|Default|SetTargetActor Target)
    (Variables|/Script/Engine.CharacterMovementComponent|SetMaxWalkSpeed (Variables|Character|GetCharacterMovement) (Variables|Default|GetAggroedMaxSpeed))
    (bind _returnvalue (Utilities|Time|SetTimerbyFunctionName self "FollowTargetDistance" 1.0 true))
    (Variables|Default|SetFollowDistanceTimer _returnvalue)
    (if (CallFunction|InAttackRange)
      (CallFunction|PerformAttack)
      (else
        (AI|AIMoveTo self "0, 0, 0" (Variables|Default|GetTargetActor) (Variables|Default|GetAtackRange) false
          (:OnSuccess
            (CallFunction|PerformAttack)))))))

(event EventBeginPlay
  (Rendering|Material|SetMaterial (Variables|Default|GetStaticMesh) 0 (Variables|Components|GetTank%20Material))
  (Variables|Default|SetStartingLocation (Transformation|GetActorLocation))
  (Variables|/Script/Engine.CharacterMovementComponent|SetMaxWalkSpeed (Variables|Character|GetCharacterMovement) (Variables|Default|GetPatrolWalkSpeed))
  (CallFunction|Patrol))

(event Collision|EventActorBeginOverlap
  (params (OtherActor :type Actor%20Object%20Reference)))

(event EventTick
  (params (DeltaSeconds :type Float%20%28single-precision%29)))

(fn ConstructionScript)

(fn InAttackRange
  (bind _targetactor (Variables|Default|GetTargetActor))
  (if (Utilities|IsValid _targetactor)
    (return (<= (Transformation|GetDistanceTo _targetactor self) (Variables|Default|GetAtackRange)))
    (else
      (return false))))

(fn GetNextAnimationIndex
  (return 0))