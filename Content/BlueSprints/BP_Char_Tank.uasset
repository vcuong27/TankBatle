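; Player tank character that drives on the yaw plane, spins its wheel meshes and fires projectiles with a muzzle effect on left click.
; Each tick, a cursor trace yaws the turret toward the aim point and places a surface-aligned decal there.
; BeginPlay applies the tank material and creates the main HUD, linking health, mana and exp bars into an enum-keyed stat map.
; UpdateStat is an unfinished stub.
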(event EventBeginPlay
  (Rendering|Material|SetMaterial (Variables|Default|GetStaticMesh) 0 (Variables|Default|GetTankMaterial))
  (bind _returnvalue (UserInterface|CreateWidget "/Game/BlueSprints/Widgets/Bp_WidgetMain.Bp_WidgetMain_C"))
  (bind _output_get (Variables|Default|SetMainWidget _returnvalue))
  (CallFunction|SetupStatBar)
  (UserInterface|Viewport|AddtoViewport _output_get 0))

(event EventTick
  (params (DeltaSeconds :type Float%20%28single-precision%29))
  (bind _returnvalue (Game|GetPlayerController 0))
  (bind _hitresult (Game|Player|GetHitResultUnderCursorbyChannel _returnvalue "TraceTypeQuery1" true))
  (bind (_bblockinghit _binitialoverlap _time _distance _location _impactpoint _normal _impactnormal) (Collision|BreakHitResult _hitresult))
  (Transformation|SetRelativeRotation (Variables|Default|GetTurtet) (Math|Rotator|MakeRotator 0.0 0.0 (- (.yaw (Math|Rotator|FindLookatRotation (Transformation|GetActorLocation) _location)) (.yaw (Transformation|GetActorRotation)))) false false)
  (Transformation|SetWorldLocationAndRotation (Variables|Default|GetDecal) _location (Math|Rotator|MakeRotationfromAxes _impactnormal "0, 0, 0" "0, 0, 0") false false))

(event Input|AxisEvents|InputAxisMoveForward
  (params (AxisValue :type Float%20%28single-precision%29))
  (if (> AxisValue 0.0)
    (CallFunction|MoveChar (* -1.0 AxisValue))
    (else
      (CallFunction|MoveChar AxisValue)))
  (Pawn|Input|AddMovementInput (Math|Vector|GetForwardVector (Math|Rotator|MakeRotator 0.0 0.0 (.Yaw (Math|Rotator|BreakRotator (Pawn|GetControlRotation :!class /Script/Engine.Pawn))))) AxisValue false))

(event Input|AxisEvents|InputAxisMoveRight
  (params (AxisValue :type Float%20%28single-precision%29))
  (if (> AxisValue 0.0)
    (CallFunction|MoveChar (* AxisValue -1.0))
    (else
      (CallFunction|MoveChar AxisValue)))
  (Pawn|Input|AddMovementInput (Math|Vector|GetRightVector (Math|Rotator|MakeRotator 0.0 0.0 (.Yaw (Math|Rotator|BreakRotator (Pawn|GetControlRotation :!class /Script/Engine.Pawn))))) AxisValue false))

(event Input|MouseEvents|LeftMouseButton
  (params (Key :type Key%20Structure :default "None"))
  (bind _spawnbullet (Variables|Default|GetSpawnBullet))
  (bind _returnvalue (Transformation|GetWorldLocation _spawnbullet))
  (:Pressed
    (Effects|SpawnEmitteratLocation "/Game/SkillFx/FX/Particles/Gideon/Abilities/Primary/FX/P_Primary_Cast.P_Primary_Cast" _returnvalue)
    (Game|SpawnActorfromClass "/Game/BlueSprints/SkillActors/Bp_ActProjectile.Bp_ActProjectile_C" (Math|Transform|MakeTransform _returnvalue (Transformation|GetWorldRotation _spawnbullet) "1,1,1") "Undefined" 0 0)))

(fn ConstructionScript)

(fn MoveChar
  (params (Speed :type Float%20%28single-precision%29))
  (Transformation|AddLocalRotation (Variables|Default|GetMDL_TankWheel_BL) (Math|Rotator|MakeRotator (* Speed (* (Variables|Default|GetSpeed) 1e+01)) 0.0 0.0) false false))

(fn GetStat
  (params (Stat :type E_Stat%20Enum :default "NewEnumerator0"))
  (return (.Value (Utilities|Map|Find (Variables|Default|GetStat) Stat))))

(fn SetStatValue
  (params (Stat :type E_Stat%20Enum :default "NewEnumerator0") (NewValue :type S%20Stat%20Data%20Structure))
  (Utilities|Map|Add (Variables|Default|GetStat) Stat NewValue)
  (return))

(fn SetupStatBar
  (bind _mainwidget (Variables|Default|GetMainWidget))
  (bind _structout (Utilities|Struct|SetmembersinS_StatData (CallFunction|GetStat "NewEnumerator1") (Variables|/Game/BlueSprints/Widgets/Bp_WidgetMain.Bp_WidgetMain_C|GetHealthBar _mainwidget)))
  (CallFunction|SetStatValue "NewEnumerator1" _structout)
  (bind _structout_2 (Utilities|Struct|SetmembersinS_StatData (CallFunction|GetStat "NewEnumerator2") (Variables|/Game/BlueSprints/Widgets/Bp_WidgetMain.Bp_WidgetMain_C|GetManaBar _mainwidget)))
  (CallFunction|SetStatValue "NewEnumerator2" _structout_2)
  (bind _structout_3 (Utilities|Struct|SetmembersinS_StatData (CallFunction|GetStat "NewEnumerator3") (Variables|/Game/BlueSprints/Widgets/Bp_WidgetMain.Bp_WidgetMain_C|GetExpBar _mainwidget)))
  (CallFunction|SetStatValue "NewEnumerator3" _structout_3))

(fn UpdateStat
  (params (Stat :type E_Stat%20Enum :default "NewEnumerator0")))